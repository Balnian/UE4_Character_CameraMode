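; BP_axe is a melee axe weapon that the player picks up by touch and that damages actors it overlaps.
; When not wielded, overlap with the player character snaps it to the Weapon_R socket on that character's mesh.
; When IsWield is true, overlaps apply CR_DamageType damage, crediting the owning CR_MainCharacter and its controller.
; The graph only reads IsWield and the owner, and sets neither on pickup.
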(event `self.ReceiveBeginPlay`)

(event `self.ReceiveActorBeginOverlap`
  (params (OtherActor :type "Actor Object Reference"))
  (bind _returnvalue (`GameplayStatics.GetPlayerCharacter` 0))
  (if (`self.IsWield`)
    (bind _ascr_main_character (cast `CR_MainCharacter` (`self.GetOwner`)))
    (`GameplayStatics.ApplyDamage` OtherActor (`self.Damage`) (`Pawn.GetController` _ascr_main_character) _ascr_main_character "/Script/Character.CR_DamageType")
    (else
      ;[1 1 1] Equip weapon
      (if (== OtherActor _returnvalue)
        (`self.K2_AttachRootComponentTo` (`Character.Mesh` _returnvalue) "Weapon_R" "SnapToTargetIncludingScale")))))

(event `self.ReceiveActorBeginOverlap`
  (params (OtherActor :type "Actor Object Reference")))

(event `self.ReceiveTick`
  (params (DeltaSeconds :type "Float (single-precision)")))

(fn `UserConstructionScript`)